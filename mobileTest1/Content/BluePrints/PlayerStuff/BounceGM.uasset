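; BounceGM, apparently a game mode by its name, respawns the player after the Player_BP pawn is destroyed.
; On BeginPlay it binds to the player pawn's OnDestroyed event.
; When that fires, it waits briefly, spawns a new Player_BP at the SpawnTransform variable and has the player controller possess it.
; It then calls Respawn to bind the new pawn, repeating the cycle for each death.
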(event Custom|OnDestroyed_Event_0
  (Utilities|FlowControl|Delay 2.0)
  (bind _returnvalue (Game|SpawnActorfromClass "/Game/BluePrints/PlayerStuff/Player_BP.Player_BP_C" (Variables|Default|GetSpawn%20Transform) false 0))
  (Pawn|Possess (Game|GetPlayerController 0) _returnvalue)
  (CallFunction|Respawn))

(event Custom|Respawn
  (bind _asplayer_bp (Utilities|Casting|CastToPlayer_BP (Game|Player|GetPlayerPawn 0)))
  (Game|BindEventtoOnDestroyed _asplayer_bp (delegate Custom|OnDestroyed_Event_0)))

(event EventBeginPlay
  (bind _asplayer_bp (Utilities|Casting|CastToPlayer_BP (Game|Player|GetPlayerPawn 0)))
  (Game|BindEventtoOnDestroyed _asplayer_bp (delegate Custom|OnDestroyed_Event_0)))

(event EventTick
  (params (DeltaSeconds :type Float%20%28single-precision%29)))

(fn ConstructionScript)