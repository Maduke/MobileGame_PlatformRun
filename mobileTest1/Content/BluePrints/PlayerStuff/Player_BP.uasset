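; Player pawn for a bounce game: a physics-driven body nudged across the world by taps.
; On BeginPlay it stores its spawn transform in BounceGM and sets a starting velocity, then each Tick orients itself along its velocity.
; Tap1 adds a fixed-strength velocity impulse horizontally toward the point under the cursor.
; Sphere hits on SpeedBoost-tagged actors roughly double velocity while below a speed cap, printing the speed.
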(event OnComponentHit(Sphere)
  (params (OtherActor :type Actor%20Object%20Reference) (OtherComp :type Primitive%20Component%20Object%20Reference) (NormalImpulse :type Vector :default "0, 0, 0") (Hit :type Hit%20Result%20Structure%20%28by%20ref%29))
  (bind _returnvalue (Transformation|GetVelocity))
  (bind _returnvalue_2 (Math|Vector|VectorLength _returnvalue))
  (if (Actor|ActorHasTag OtherActor "SpeedBoost")
    (if (< (* _returnvalue_2 2.0) 2.5e+03)
      (Physics|SetPhysicsLinearVelocity (* _returnvalue 1.1) true "None")
      (Development|PrintString (Utilities|String|ToString(Float) _returnvalue_2)))))

(event EventTick
  (params (DeltaSeconds :type Float%20%28single-precision%29))
  (Transformation|SetWorldRotation (Math|Rotator|MakeRotationfromAxes (Transformation|GetVelocity) "0, 0, 0" "0, 0, 0") false))

(event EventBeginPlay
  (bind _asbounce_gm (Utilities|Casting|CastToBounceGM (Game|GetGameMode)))
  (Variables|/Game/BluePrints/PlayerStuff/BounceGM.BounceGM_C|SetSpawn%20Transform _asbounce_gm (Transformation|GetActorTransform))
  (Physics|SetPhysicsLinearVelocity "0,-100.000000, 0" false "None"))

(event EventActorBeginOverlap
  (params (OtherActor :type Actor%20Object%20Reference)))

(event Input|ActionEvents|InputActionTap1
  (bind _returnvalue (Game|GetPlayerController 0))
  (bind _hitresult (Game|Player|GetHitResultUnderCursorbyChannel _returnvalue "TraceTypeQuery1" true))
  (bind _location (Collision|BreakHitResult _hitresult))
  (bind (_x _y) (Math|Vector|BreakVector _location))
  (:Pressed
    (Physics|AddImpulse (Math|Vector|RotateVector "250.000000,0.000000,0.000000" (Class|KismetMathLibrary|MakeRot 0.0 (.Yaw (Class|KismetMathLibrary|BreakRot (Math|Rotator|FindLookatRotation (Transformation|GetActorLocation) (Math|Vector|MakeVector _x _y 0.0)))) 0.0)) "None" true)))

(fn ConstructionScript)