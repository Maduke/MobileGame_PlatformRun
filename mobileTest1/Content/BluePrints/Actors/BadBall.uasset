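; BadBall is an enemy physics ball that chases the player using velocity-change impulses.
; A Tick-driven state machine uses Delay nodes to pace small nudges toward the player pawn, counting up to twenty.
; It then leaps up and toward the world's XY origin, waits, and launches a hard charge at the player before repeating.
; MoveToPlayer flattens the look-at to the ball's height, keeping pursuit impulses horizontal.
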(event EventBeginPlay)

(event EventActorBeginOverlap
  (params (OtherActor :type Actor%20Object%20Reference)))

(event EventTick
  (params (DeltaSeconds :type Float%20%28single-precision%29))
  (bind _returnvalue (Transformation|GetActorLocation))
  (bind (_x _y _z) (Math|Vector|BreakVector _returnvalue))
  (Utilities|FlowControl|Sequence
    (:then_0
      (if (>= (Variables|Default|Getact) 20)
        (Variables|Default|Setact 0)
        (Variables|Default|SetAction 1)))
    (:then_1
      (if (== (Variables|Default|GetAction) 0)
        (Utilities|FlowControl|Delay 0.2)
        (Variables|Default|Setact (+ (Variables|Default|Getact) 1))
        (CallFunction|MovetoPlayer 1e+02)))
    (:then_2
      (if (== (Variables|Default|GetAction) 1)
        (Physics|AddImpulse (Math|Vector|RotateVector "600.000000, 0,500.000000" (Math|Rotator|FindLookatRotation (Math|Vector|MakeVector _x _y _z) (Math|Vector|MakeVector 0.0 0.0 _z))) "None" true)
        (Variables|Default|SetAction 2)))
    (:then_3
      (if (== (Variables|Default|GetAction) 2)
        (Utilities|FlowControl|Delay 3.0)
        (CallFunction|MovetoPlayer 2e+03)
        (Variables|Default|SetAction 0)))))

(fn ConstructionScript)

(fn MovetoPlayer
  (params (Magnitude :type Float%20%28single-precision%29 :default 0.0))
  (bind _returnvalue (Transformation|GetActorLocation))
  (bind _returnvalue_2 (Game|Player|GetPlayerPawn 0))
  (bind (_x _y _z) (Math|Vector|BreakVector _returnvalue))
  (bind _returnvalue_3 (Transformation|GetActorLocation _returnvalue_2))
  (bind (_x_2 _y_2) (Math|Vector|BreakVector _returnvalue_3))
  ;[1 1 1] Go Towards Player
  (Physics|AddImpulse (Math|Vector|RotateVector (Math|Vector|MakeVector Magnitude 0.0 0.0) (Math|Rotator|FindLookatRotation (Math|Vector|MakeVector _x _y _z) (Math|Vector|MakeVector _x_2 _y_2 _z))) "None" true))